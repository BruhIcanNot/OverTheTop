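; Trap floor that rattles, vanishes and respawns after the player character steps on it.
; Overlapping the Box trigger plays the Rattle timeline, shifting the Cube along its right vector and rolling it around its starting location.
; A parallel reset chain hides the Cube and disables collision on it and the trigger after a short delay, then restores both after PlatformRespawnTimer and stops the timeline.
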(event OnComponentBeginOverlap(Box)
  (params (OverlappedComponent :type Primitive%20Component%20Object%20Reference) (OtherActor :type Actor%20Object%20Reference) (OtherComp :type Primitive%20Component%20Object%20Reference) (OtherBodyIndex :type Integer) (bFromSweep :type Boolean) (SweepResult :type Hit%20Result%20Structure%20%28by%20ref%29))
  (bind _cube (Variables|Default|GetCube))
  (Utilities|Casting|CastToBP_ThirdPersonCharacter OtherActor)
  (CallFunction|ResetLoop)
  (bind _newtrack_0 (Timeline|Rattle PlayFromStart)
    (:Update
      (Transformation|SetRelativeLocation _cube (+ (Variables|Default|GetOGLocation) (* (* (Math|Vector|GetRightVector (Variables|Default|GetCube)) _newtrack_0) 1e+01)) false false)
      (Transformation|SetRelativeRotation _cube (Math|Rotator|MakeRotator (* _newtrack_0 8.0) 0.0 0.0) false false))))

(event Custom|ResetLoop
  (bind _cube (Variables|Default|GetCube))
  (Utilities|FlowControl|Delay 1.0)
  (Rendering|SetVisibility (Variables|Default|GetCube) false false)
  (Collision|SetCollisionEnabled (Variables|Default|GetBox) "NoCollision")
  (Utilities|FlowControl|Delay (Variables|Default|GetPlatformRespawnTimer))
  (Rendering|SetVisibility (Variables|Default|GetCube) true false)
  (Collision|SetCollisionEnabled (Variables|Default|GetBox) "QueryAndPhysics")
  (bind _newtrack_0 (Timeline|Rattle Stop)
    (:Update
      (Transformation|SetRelativeLocation _cube (+ (Variables|Default|GetOGLocation) (* (* (Math|Vector|GetRightVector (Variables|Default|GetCube)) _newtrack_0) 1e+01)) false false)
      (Transformation|SetRelativeRotation _cube (Math|Rotator|MakeRotator (* _newtrack_0 8.0) 0.0 0.0) false false))))

(event EventBeginPlay
  (bind _cube (Variables|Default|GetCube))
  (Variables|Default|SetOGLocation (Variables|/Script/Engine.SceneComponent|GetRelativeLocation _cube))
  (Variables|Default|SetOGRotation (Variables|/Script/Engine.SceneComponent|GetRelativeRotation _cube)))

(fn ConstructionScript)