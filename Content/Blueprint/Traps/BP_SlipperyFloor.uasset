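; BP_SlipperyFloor is an ice floor trap that makes player 0's character slide.
; Box overlap sets an OnIce flag and lowers the character's ground friction, braking and acceleration, restoring hard-coded values on exit.
; Tick forces forward movement input while OnIce and the BP_ThirdPersonCharacter's IsIdlingOnIce are both true.
; Overlap handlers always modify player 0, without checking which actor overlapped.
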(event OnComponentBeginOverlap(Box)
  (params (OverlappedComponent :type Primitive%20Component%20Object%20Reference) (OtherActor :type Actor%20Object%20Reference) (OtherComp :type Primitive%20Component%20Object%20Reference) (OtherBodyIndex :type Integer) (bFromSweep :type Boolean) (SweepResult :type Hit%20Result%20Structure%20%28by%20ref%29))
  (bind _returnvalue (Game|GetPlayerCharacter 0))
  (bind _charactermovement (Variables|/Script/Engine.Character|GetCharacterMovement _returnvalue))
  (Variables|Default|SetOnIce true)
  (Variables|/Script/Engine.CharacterMovementComponent|SetGroundFriction _charactermovement 0.0)
  (Variables|/Script/Engine.CharacterMovementComponent|SetBrakingDecelerationWalking _charactermovement 2e+02)
  (Variables|/Script/Engine.CharacterMovementComponent|SetMaxAcceleration _charactermovement 4e+02))

(event OnComponentEndOverlap(Box)
  (params (OverlappedComponent :type Primitive%20Component%20Object%20Reference) (OtherActor :type Actor%20Object%20Reference) (OtherComp :type Primitive%20Component%20Object%20Reference) (OtherBodyIndex :type Integer))
  (bind _returnvalue (Game|GetPlayerCharacter 0))
  (bind _charactermovement (Variables|/Script/Engine.Character|GetCharacterMovement _returnvalue))
  (Variables|Default|SetOnIce false)
  (Variables|/Script/Engine.CharacterMovementComponent|SetGroundFriction _charactermovement 8.0)
  (Variables|/Script/Engine.CharacterMovementComponent|SetBrakingDecelerationWalking _charactermovement 1e+04)
  (Variables|/Script/Engine.CharacterMovementComponent|SetMaxAcceleration _charactermovement 1.5e+03))

(event EventBeginPlay
  (bind _asbp_third_person_character (Utilities|Casting|CastToBP_ThirdPersonCharacter (Game|GetPlayerCharacter 0)))
  (Variables|Default|SetPlayerREF _asbp_third_person_character))

(event Collision|EventActorBeginOverlap
  (params (OtherActor :type Actor%20Object%20Reference)))

(event EventTick
  (params (DeltaSeconds :type Float%20%28single-precision%29))
  (bind _returnvalue (Game|GetPlayerCharacter 0))
  (if (and (Variables|/Game/ThirdPerson/Blueprints/BP_ThirdPersonCharacter.BP_ThirdPersonCharacter_C|GetisIdlingOnIce (Variables|Default|GetPlayerREF)) (Variables|Default|GetOnIce))
    (Pawn|Input|AddMovementInput _returnvalue (Transformation|GetActorForwardVector _returnvalue) 0.3 true)))

(fn ConstructionScript)