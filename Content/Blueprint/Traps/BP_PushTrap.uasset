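; BP_PushTrap is a trap that slides a cube sideways and shoves the player character with a strong launch.
; On BeginPlay a timeline, with adjustable play rate, lerps the cube from its starting relative location along the right vector by Distance, without sweep.
; Separately, when a BP_ThirdPersonCharacter overlaps the Box, player 0's character receives a fixed, additive launch along world +Y, independent of the cube's motion.
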(event OnComponentBeginOverlap(Box)
  (params (OverlappedComponent :type Primitive%20Component%20Object%20Reference) (OtherActor :type Actor%20Object%20Reference) (OtherComp :type Primitive%20Component%20Object%20Reference) (OtherBodyIndex :type Integer) (bFromSweep :type Boolean) (SweepResult :type Hit%20Result%20Structure%20%28by%20ref%29))
  (Utilities|Casting|CastToBP_ThirdPersonCharacter OtherActor)
  (Character|LaunchCharacter (Game|GetPlayerCharacter 0) "0.000000,6200.000000,0.000000" false false))

(event EventBeginPlay
  (Variables|Default|SetOGLocation (Variables|/Script/Engine.SceneComponent|GetRelativeLocation (Variables|Default|GetCube1)))
  (Components|Timeline|SetPlayRate (Variables|Default|GetTimeline) (Variables|Default|GetTimeLineSpeed))
  (bind _newtrack_0 (Timeline|Timeline PlayFromStart)
    (:Update
      (Transformation|SetRelativeLocation (Variables|Default|GetCube1) (Math|Vector|Lerp(Vector) (Variables|Default|GetOGLocation) (+ (Variables|Default|GetOGLocation) (* (Class|KismetMathLibrary|VectorRight) (Variables|Default|GetDistance))) _newtrack_0) false false))))

(event Collision|EventActorBeginOverlap
  (params (OtherActor :type Actor%20Object%20Reference)))

(fn ConstructionScript)